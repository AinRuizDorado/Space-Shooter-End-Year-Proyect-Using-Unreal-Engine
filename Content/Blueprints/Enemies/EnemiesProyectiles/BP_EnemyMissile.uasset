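; BP_EnemyMissile is an enemy missile projectile with randomized speed and size that awards score when killed.
; BeginPlay caches BP_GameMode, sets projectile movement speed and scales the mesh randomly per axis within min/max ranges.
; Tick reapplies a fixed 90-degree pitch and that scale to the actor at its current location.
; EnemyKilled passes its score value to the game mode; camera shake, sound and destroy nodes are left unconnected.
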(event `self.ReceiveBeginPlay`
  (bind _projectilemovement (`self.ProjectileMovement`))
  (bind _returnvalue (`KismetMathLibrary.RandomFloatInRange` (`self.MinScale`) (`self.MaxScale`)))
  (bind _asbp_game_mode (cast `/Game/Blueprints/BP_GameMode` (`GameplayStatics.GetGameMode`)))
  (set `self.BP Game mode` _asbp_game_mode)
  (bind _output_get (set `self.MoveSpeed` (`KismetMathLibrary.RandomFloatInRange` (`self.MinSpeed`) (`self.MaxSpeed`))))
  (bind _output_get_2 (set `ProjectileMovementComponent.MaxSpeed` _output_get _projectilemovement))
  (set `ProjectileMovementComponent.InitialSpeed` _output_get_2 _projectilemovement)
  (bind _output_get_3 (set `self.Scale` (`KismetMathLibrary.MakeVector` _returnvalue _returnvalue _returnvalue)))
  (`SceneComponent.SetWorldScale3D` (`self.StaticMesh`) _output_get_3))

(event `self.ReceiveTick`
  (params (DeltaSeconds :type "Float (single-precision)"))
  (`self.K2_SetActorTransform` (`KismetMathLibrary.MakeTransform` (`self.K2_GetActorLocation`) (`KismetMathLibrary.MakeRotator` 0.0 90.0) (`self.Scale`))))

(event `self.EnemyKilled`
  (`/Game/Blueprints/BP_GameMode.SetScore` (`self.BP_GameMode`) (`self.Enemy Score Value`)))

(fn `UserConstructionScript`
  (`parent.UserConstructionScript`)
  (`SceneComponent.SetWorldScale3D` (`self.StaticMesh`) (`self.Scale`)))