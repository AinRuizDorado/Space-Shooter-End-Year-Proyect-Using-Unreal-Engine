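; Player pawn for a shooter that moves in the X/Z plane, fires two projectile weapons and triggers game over on death.
; A spawn timeline lifts and spins it before enabling firing.
; Axis inputs ease velocities that Tick applies as swept offsets with yaw following horizontal speed, while box hits redirect them along the normal.
; Looping timers repeat fire while held, and damage shakes the camera through BP_GameMode, exploding the player at zero health.
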(event `self.ReceiveBeginPlay`
  (bind _spawnlocation (`self.SpawnLocation`))
  ;[1 1 1] Player Spawn
  (bind _asbp_game_mode (cast `/Game/Blueprints/BP_GameMode` (`GameplayStatics.GetGameMode`)))
  (set `self.BP_GameMode` _asbp_game_mode)
  (set `self.Yaw` (.yaw (`self.K2_GetActorRotation`)))
  (set `self.SpawnLocation` (`self.K2_GetActorLocation`))
  (bind (_direction _speed) (`Timeline|SpawnAnimation`)
    (:`Update`
      (`self.K2_SetActorLocation` (`KismetMathLibrary.VLerp` _spawnlocation (+ _spawnlocation (0.0 0.0 60.0)) _speed))
      ;;[1 1 1] Bug de colision
      (`SceneComponent.K2_SetRelativeRotation` (`self.PlayerMesh`) (`KismetMathLibrary.RLerp` (struct) (`KismetMathLibrary.MakeRotator` 0.0 0.0 (+ (`self.Yaw`) (`self.Spawn Spin Count`))) _speed) false false))
    (:`Finished`
      (set `self.MoveEnabled` true))))

(event `self.ReceiveTick`
  (params (DeltaSeconds :type "Float (single-precision)"))
  (bind _playermesh (`self.PlayerMesh`))
  ;[1 1 1] Movement
  (set `self.DeltaSeconds` DeltaSeconds)
  (`self.K2_SetActorLocation` (+ (`self.K2_GetActorLocation`) (`KismetMathLibrary.MakeVector` (`self.HozSpeed`))) true)
  (`self.K2_SetActorLocation` (+ (`self.K2_GetActorLocation`) (`KismetMathLibrary.MakeVector` 0.0 0.0 (`self.VertSpeed`))) true)
  (`/Engine/EditorBlueprintResources/StandardMacros.IsValid` self
    (:`Is Valid`
      (`SceneComponent.K2_SetRelativeRotation` _playermesh (`KismetMathLibrary.RInterpTo` (`SceneComponent.RelativeRotation` _playermesh) (`KismetMathLibrary.MakeRotator` 0.0 0.0 (+ (* (`self.HozSpeed`) -7.0) (`self.Yaw`))) (`self.DeltaSeconds`) 80.0) false false))))

(event `InputAxis|MoveRight`
  (params (AxisValue :type "Float (single-precision)"))
  ;[1 1 1] Speed Movement
  (bind _returndirectionspeed (`self.Movement` AxisValue (`self.HozSpeed`)))
  (set `self.HozSpeed` _returndirectionspeed))

(event `InputAxis|MoveUp`
  (params (AxisValue :type "Float (single-precision)"))
  ;[1 1 1] Speed Movement
  (bind _returndirectionspeed (`self.Movement` AxisValue (`self.VertSpeed`)))
  (set `self.VertSpeed` _returndirectionspeed))

(event `self.ReceiveAnyDamage`
  (params (Damage :type "Float (single-precision)") (DamageType :type "DamageType Object Reference") (InstigatedBy :type "Controller Object Reference") (DamageCauser :type "Actor Object Reference"))
  (bind _bp_gamemode (`self.BP_GameMode`))
  ;[1 1 1] Game Over
  (set `self.Health` (`KismetMathLibrary.FClamp` (- (`self.Health`) Damage) 0.0 (`self.MaxHealth`)))
  (`/Game/Blueprints/BP_GameMode.PlayCamShake` (`self.BP_GameMode`) "/Script/Engine.CameraShake" (`self.K2_GetActorLocation`))
  (if (<= (`self.Health`) 0.0)
    (`GameplayStatics.SpawnEmitterAtLocation` "/Game/Assets/Particules/P_Pixel_Explosion_Player.P_Pixel_Explosion_Player" (`self.K2_GetActorLocation`))
    (`GameplayStatics.PlaySoundAtLocation` null)
    (`/Game/Blueprints/BP_GameMode.PlayCamShake` _bp_gamemode "/Script/Engine.CameraShake" (`self.K2_GetActorLocation`))
    (`/Game/Blueprints/BP_GameMode.Game Over` _bp_gamemode)
    (`self.K2_DestroyActor`)))

(event `PrimFire`
  ;[1 1 1] PrimaryFire
  (`self.PrimaryFire` (`SceneComponent.K2_GetComponentToWorld` (`self.ProjectileSpawn`)) :!label _label))

(event `InputAction|PrimaryFire`
  (params (Key :type "Key Structure"))
  ;[1 1 1] PrimaryFire
  (:`Pressed`
    (if (`self.MoveEnabled`)
      (`KismetSystemLibrary.K2_SetTimer` null "PrimFire" 0.6 true)
      (goto _label)))
  (:`Released`
    (`KismetSystemLibrary.K2_ClearTimer` null "PrimFire")))

(event `SecFire`
  ;[1 1 1] Secondary Fire
  (`self.Secondary Fire` (`SceneComponent.K2_GetComponentToWorld` (`self.ProyectileSpawnZ`)) :!label _label_2)
  (`self.Secondary Fire` (`SceneComponent.K2_GetComponentToWorld` (`self.PryectileSpawnX`))))

(event `InputAction|SecondaryFire`
  (params (Key :type "Key Structure"))
  ;[1 1 1] Secondary Fire
  (:`Pressed`
    (if (`self.MoveEnabled`)
      (`KismetSystemLibrary.K2_SetTimer` null "SecFire" 0.2 true)
      (goto _label_2)))
  (:`Released`
    (`KismetSystemLibrary.K2_ClearTimer` null "SecFire")))

(event `self.Box.OnComponentHit`
  (params (HitComponent :type "PrimitiveComponent Object Reference") (OtherActor :type "Actor Object Reference") (OtherComp :type "PrimitiveComponent Object Reference") (NormalImpulse :type "Vector Structure") (Hit :type "HitResult Structure (by ref)"))
  (set `self.HozSpeed` (* (* (`KismetMathLibrary.Abs` (`self.HozSpeed`)) 1.0) (.x Hit_Normal)))
  (set `self.VertSpeed` (* (* (`KismetMathLibrary.Abs` (`self.VertSpeed`)) 1.0) (.z Hit_Normal))))

(fn `Movement`
  (params (Direction :type "Float (double-precision)") (Speed :type "Float (double-precision)"))
  (returns (ReturnDirectionSpeed :type "Float (double-precision)"))
  (return (`KismetMathLibrary.FInterpTo` Speed (* (* Direction (`self.MovementSpeed`)) (`self.DeltaSeconds`)) (`self.DeltaSeconds`) 6.0)))

(fn `PrimaryFire`
  (params (SpawnTransform :type "Transform Structure"))
  (locals (`Projectile Color` :type "LinearColor Structure" :default (struct)) (proyectileColour :type "LinearColor Structure" :default (struct :`R` 0.017323 :`G` 0.05657 :`B` 0.845)))
  (`|SpawnActorFromClass` "/Game/Blueprints/BP_Proyectiles/BP_Player_ProyectilePrimary.BP_Player_ProyectilePrimary_C" SpawnTransform "AlwaysSpawn" "OverrideRootScale" null (`local.proyectileColour`) self))

(fn `Secondary Fire`
  (params (Spawn :type "Transform Structure"))
  (locals (Colour :type "LinearColor Structure" :default (struct :`R` 1.0 :`B` 0.009094)))
  (`|SpawnActorFromClass` "/Game/Blueprints/BP_Proyectiles/BP_Player_ProyectileSecondary.BP_Player_ProyectileSecondary_C" Spawn "AlwaysSpawn" "OverrideRootScale" null (`local.Colour`) null))

(fn `UserConstructionScript`
  (set `self.Health` (`self.MaxHealth`)))