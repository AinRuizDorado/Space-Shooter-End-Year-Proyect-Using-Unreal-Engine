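; Player pawn for a shooter that moves on the X/Z plane and fires primary and secondary projectiles.
; BeginPlay plays a timeline that raises and spins it in, then sets MoveEnabled, which gates firing but not movement.
; Axis inputs interpolate speeds that Tick applies as swept per-frame offsets, yawing the mesh with horizontal speed.
; Held fire repeats on looping timers, with secondary fire spawning from two points.
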(event `self.ReceiveBeginPlay`
  (bind _spawnlocation (`self.SpawnLocation`))
  ;[1 1 1] Player Spawn
  (bind _asbp_game_mode (cast `/Game/Blueprints/BP_GameMode` (`GameplayStatics.GetGameMode`)))
  (set `self.BP_GameMode` _asbp_game_mode)
  (set `self.Yaw` (.yaw (`self.K2_GetActorRotation`)))
  (set `self.SpawnLocation` (`self.K2_GetActorLocation`))
  (bind (_direction _speed) (`Timeline|SpawnAnimation`)
    (:`Update`
      (`self.K2_SetActorLocation` (`KismetMathLibrary.VLerp` _spawnlocation (+ _spawnlocation (0.0 0.0 60.0)) _speed))
      ;;[1 1 1] Bug de colision
      (`SceneComponent.K2_SetRelativeRotation` (`self.PlayerMesh`) (`KismetMathLibrary.RLerp` (struct) (`KismetMathLibrary.MakeRotator` 0.0 0.0 (+ (`self.Yaw`) (`self.Spawn Spin Count`))) _speed) false false))
    (:`Finished`
      (set `self.MoveEnabled` true))))

(event `self.ReceiveTick`
  (params (DeltaSeconds :type "Float (single-precision)"))
  (bind _playermesh (`self.PlayerMesh`))
  ;[1 1 1] Movement
  (set `self.DeltaSeconds` DeltaSeconds)
  (`self.K2_SetActorLocation` (+ (`self.K2_GetActorLocation`) (`KismetMathLibrary.MakeVector` (`self.HozSpeed`))) true)
  (`self.K2_SetActorLocation` (+ (`self.K2_GetActorLocation`) (`KismetMathLibrary.MakeVector` 0.0 0.0 (`self.VertSpeed`))) true)
  (`SceneComponent.K2_SetRelativeRotation` _playermesh (`KismetMathLibrary.RInterpTo` (`SceneComponent.RelativeRotation` _playermesh) (`KismetMathLibrary.MakeRotator` 0.0 0.0 (+ (* (`self.HozSpeed`) -20.0) (`self.Yaw`))) (`self.DeltaSeconds`) 80.0) false false))

(event `InputAxis|MoveRight`
  (params (AxisValue :type "Float (single-precision)"))
  ;[1 1 1] Speed Movement
  (bind _returndirectionspeed (`self.Movement` AxisValue (`self.HozSpeed`)))
  (set `self.HozSpeed` _returndirectionspeed))

(event `InputAxis|MoveUp`
  (params (AxisValue :type "Float (single-precision)"))
  ;[1 1 1] Speed Movement
  (bind _returndirectionspeed (`self.Movement` AxisValue (`self.VertSpeed`)))
  (set `self.VertSpeed` _returndirectionspeed))

(event `PrimFire`
  ;[1 1 1] PrimaryFire
  (`self.PrimaryFire` (`SceneComponent.K2_GetComponentToWorld` (`self.ProjectileSpawn`)) :!label _label))

(event `InputAction|PrimaryFire`
  (params (Key :type "Key Structure"))
  ;[1 1 1] PrimaryFire
  (:`Pressed`
    (if (`self.MoveEnabled`)
      (`KismetSystemLibrary.K2_SetTimer` null "PrimFire" 0.2 true)
      (goto _label)))
  (:`Released`
    (`KismetSystemLibrary.K2_ClearTimer` null "PrimFire")))

(event `SecFire`
  ;[1 1 1] Secondary Fire
  (`self.Secondary Fire` (`SceneComponent.K2_GetComponentToWorld` (`self.ProyectileSpawnZ`)) :!label _label_2)
  (`self.Secondary Fire` (`SceneComponent.K2_GetComponentToWorld` (`self.PryectileSpawnX`))))

(event `InputAction|SecondaryFire`
  (params (Key :type "Key Structure"))
  ;[1 1 1] Secondary Fire
  (:`Pressed`
    (if (`self.MoveEnabled`)
      (`KismetSystemLibrary.K2_SetTimer` null "SecFire" 0.6 true)
      (goto _label_2)))
  (:`Released`
    (`KismetSystemLibrary.K2_ClearTimer` null "SecFire")))

(fn `Movement`
  (params (Direction :type "Float (double-precision)") (Speed :type "Float (double-precision)"))
  (returns (ReturnDirectionSpeed :type "Float (double-precision)"))
  (return (`KismetMathLibrary.FInterpTo` Speed (+ (`self.MovementSpeed`) Direction) (`self.DeltaSeconds`) 6.0)))

(fn `PrimaryFire`
  (params (SpawnTransform :type "Transform Structure"))
  (locals (`Projectile Color` :type "LinearColor Structure" :default (struct)) (proyectileColour :type "LinearColor Structure" :default (struct :`R` 0.017323 :`G` 0.05657 :`B` 0.845)))
  (`|SpawnActorFromClass` "/Game/Blueprints/BP_Proyectiles/BP_Player_ProyectilePrimary.BP_Player_ProyectilePrimary_C" SpawnTransform "AlwaysSpawn" "OverrideRootScale" null (`local.proyectileColour`) self))

(fn `Secondary Fire`
  (params (Spawn :type "Transform Structure"))
  (locals (Colour :type "LinearColor Structure" :default (struct :`R` 1.0 :`B` 0.009094)))
  (`|SpawnActorFromClass` "/Game/Blueprints/BP_Proyectiles/BP_Player_ProyectileSecondary.BP_Player_ProyectileSecondary_C" Spawn "AlwaysSpawn" "OverrideRootScale" null (`local.Colour`) null))

(fn `UserConstructionScript`
  (set `self.Health` (`self.MaxHealth`)))