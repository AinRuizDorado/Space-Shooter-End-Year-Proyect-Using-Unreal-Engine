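; Base enemy projectile Blueprint that flies via ProjectileMovement and damages the player on impact.
; The construction script creates a dynamic material for the mesh and applies the configured scale and speed.
; BeginPlay tints that material with the projectile colour.
; On any mesh hit it applies damage if the other actor is BP_Player, then destroys itself.
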(event `self.ReceiveBeginPlay`
  (`MaterialInstanceDynamic.SetVectorParameterValue` (`self.ProyectileMaterial`) "Colour" (`self.Proyectile Color`)))

(event `self.StaticMesh.OnComponentHit`
  (params (HitComponent :type "PrimitiveComponent Object Reference") (OtherActor :type "Actor Object Reference") (OtherComp :type "PrimitiveComponent Object Reference") (NormalImpulse :type "Vector Structure") (Hit :type "HitResult Structure (by ref)"))
  (cast `/Game/Blueprints/BP_Player` OtherActor
    (:`then`
      (`GameplayStatics.ApplyDamage` null (`self.Damage`)))
    (:`CastFailed`
      _))
  (`self.K2_DestroyActor`))

(fn `UserConstructionScript`
  (bind _projectilemovement (`self.ProjectileMovement`))
  (bind _returnvalue (`PrimitiveComponent.CreateDynamicMaterialInstance` (`self.StaticMesh`) 0 null))
  (set `self.ProyectileMaterial` _returnvalue)
  (`SceneComponent.SetWorldScale3D` (`self.StaticMesh`) (`self.Scale`))
  (bind _output_get (set `ProjectileMovementComponent.MaxSpeed` (`self.Speed`) _projectilemovement))
  (set `ProjectileMovementComponent.InitialSpeed` _output_get _projectilemovement))