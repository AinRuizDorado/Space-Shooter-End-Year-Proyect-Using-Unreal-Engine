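; BP_EnemyMissile is an enemy missile actor that holds a fixed vertical orientation, pitched 90 degrees.
; Each Tick calls the parent, then rewrites the actor transform with its current location, that constant rotation and the Scale variable, without sweeping.
; The construction script also applies Scale to the static mesh's world scale.
; The graph itself contains no movement, overlap or damage logic.
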(event `self.ReceiveTick`
  (params (DeltaSeconds :type "Float (single-precision)"))
  (`parent.ReceiveTick` DeltaSeconds)
  (`self.K2_SetActorTransform` (`KismetMathLibrary.MakeTransform` (`self.K2_GetActorLocation`) (`KismetMathLibrary.MakeRotator` 0.0 90.0) (`self.Scale`))))

(fn `UserConstructionScript`
  (`parent.UserConstructionScript`)
  (`SceneComponent.SetWorldScale3D` (`self.StaticMesh`) (`self.Scale`)))