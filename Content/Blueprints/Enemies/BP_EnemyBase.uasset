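; BP_EnemyBase is a base enemy actor that drops in at spawn and then moves horizontally along the world X axis.
; BeginPlay adds one to the BP_GameMode enemy count, then picks a random direction and a speed between MinSpeed and MaxSpeed.
; A timeline lerps it 120 units down from its spawn location, then enables movement.
; Tick applies frame-rate-independent movement by setting the location directly, without sweep.
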(event `self.ReceiveBeginPlay`
  (bind _spawn_location (`self.Spawn Location`))
  ;[1 1 1] Setup variables and interance
  (bind _asbp_game_mode (cast `/Game/Blueprints/BP_GameMode` (`GameplayStatics.GetGameMode`)))
  (bind _output_get (set `self.BP Game mode` _asbp_game_mode))
  (`/Game/Blueprints/BP_GameMode.Update Enemy Count` _output_get 1)
  (set `self.MoveDirection` (`KismetMathLibrary.RandomBool`))
  (set `self.MoveSpeed` (`KismetMathLibrary.RandomFloatInRange` (`self.MinSpeed`) (`self.MaxSpeed`)))
  (set `self.Spawn Location` (`self.K2_GetActorLocation`))
  ;[1 1 1] Spawn Animation
  (bind (_direction _entryspeed) (`Timeline|SpawnAnimatin` :`NewTime` 0.0)
    (:`Update`
      (`self.K2_SetActorLocation` (`KismetMathLibrary.VLerp` _spawn_location (- _spawn_location (0.0 0.0 120.0)) _entryspeed)))
    (:`Finished`
      (set `self.MoveEnabled` true))))

(event `self.ReceiveTick`
  (params (DeltaSeconds :type "Float (single-precision)"))
  (if (`self.MoveEnabled`)
    (`self.K2_SetActorLocation` (+ (`self.K2_GetActorLocation`) (* (`KismetMathLibrary.MakeVector` (* (`self.MoveSpeed`) (`KismetMathLibrary.SelectFloat` 1.0 -1.0 (`self.MoveDirection`)))) DeltaSeconds)))))

(fn `UserConstructionScript`)