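; Base Blueprint for player projectiles, with configurable colour, scale, speed and damage.
; The construction script creates a dynamic material instance, scales the mesh and sets the projectile movement's initial and max speed.
; BeginPlay tints the material with the projectile colour.
; On any overlap it applies damage to the other actor, spawns a pixel explosion particle and destroys itself.
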(event `self.ReceiveBeginPlay`
  (`MaterialInstanceDynamic.SetVectorParameterValue` (`self.Proyectile Material`) "Colour" (`self.ProyectileColor`)))

(event `self.Proyectile.OnComponentBeginOverlap`
  (params (OverlappedComponent :type "PrimitiveComponent Object Reference") (OtherActor :type "Actor Object Reference") (OtherComp :type "PrimitiveComponent Object Reference") (OtherBodyIndex :type Integer) (bFromSweep :type Boolean) (SweepResult :type "HitResult Structure (by ref)"))
  (`GameplayStatics.ApplyDamage` OtherActor (`self.Damage`))
  (`GameplayStatics.SpawnEmitterAtLocation` "/Game/Assets/Particules/P_Pixel_Explosion.P_Pixel_Explosion" (`self.K2_GetActorLocation`))
  (`self.K2_DestroyActor`))

(fn `UserConstructionScript`
  (bind _projectilemovement (`self.ProjectileMovement`))
  (bind _returnvalue (`PrimitiveComponent.CreateDynamicMaterialInstance` (`self.Proyectile`) 0 null))
  (set `self.Proyectile Material` _returnvalue)
  (`SceneComponent.SetWorldScale3D` (`self.Proyectile`) (`self.Scale`))
  (bind _output_get (set `ProjectileMovementComponent.MaxSpeed` (`self.Speed`) _projectilemovement))
  (set `ProjectileMovementComponent.InitialSpeed` _output_get _projectilemovement))