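; BP_Player_Proyectile is a player projectile with configurable color, scale and speed, moved by a ProjectileMovement component.
; The construction script creates a dynamic material on the Proyectile component, sets its world scale and applies Speed as MaxSpeed.
; BeginPlay writes ProyectileColor to the material's "color" parameter.
; The node copying MaxSpeed into InitialSpeed is disconnected, so InitialSpeed is not set here.
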(event `self.ReceiveBeginPlay`
  (`MaterialInstanceDynamic.SetVectorParameterValue` (`self.ProyectileMaterial`) "color" (`self.ProyectileColor`)))

(fn `UserConstructionScript`
  (bind _returnvalue (`PrimitiveComponent.CreateDynamicMaterialInstance` (`self.Proyectile`) 0 null))
  (set `self.ProyectileMaterial` _returnvalue)
  (`SceneComponent.SetWorldScale3D` (`self.Proyectile`) (`self.Scale`))
  (bind _output_get (set `ProjectileMovementComponent.MaxSpeed` (`self.Speed`) (`self.ProjectileMovement`))))